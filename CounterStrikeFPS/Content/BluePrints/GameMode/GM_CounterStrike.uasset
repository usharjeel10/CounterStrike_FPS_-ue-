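; GM_CounterStrike is a game mode that tracks joining players and spawns them at team spawn points for Counter-Terrorists or Terrorists.
; On each PostLogin it records the player controller and refreshes the arrays of spawn point actors for both teams.
; A team request calls SpawnPlayer on the controller with the chosen class and a random spawn transform from the matching team.
; A getter returns the game mode itself.
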(event `self.K2_PostLogin`
  (params (NewPlayer :type "PlayerController Object Reference"))
  (`KismetArrayLibrary.Array_AddUnique` (`self.PlayerCollected`) NewPlayer)
  (bind _outactors (`GameplayStatics.GetAllActorsOfClass` "/Game/BluePrints/SpawnPoints/BP_SP_CounterTerrorist.BP_SP_CounterTerrorist_C"))
  (set `self.counterTerroristPos` _outactors)
  (bind _outactors_2 (`GameplayStatics.GetAllActorsOfClass` "/Game/BluePrints/SpawnPoints/BP_SP_Terrorist.BP_SP_Terrorist_C"))
  (set `self.TerroristPos` _outactors_2))

(event `requestTeam`
  (params (playerController :type "/Game/BluePrints/PlayerController/PC_CounterStrike Object Reference") (Class :type "Actor Class Reference"))
  (`/Game/BluePrints/PlayerController/PC_CounterStrike.spawnPlayer` playerController Class (`KismetMathLibrary.SelectTransform` (`self.GetTransform` (`KismetArrayLibrary.Array_Random` (`self.counterTerroristPos`))) (`self.GetTransform` (`KismetArrayLibrary.Array_Random` (`self.TerroristPos`))) (== Class "/Game/BluePrints/Characters/BP_CounterTerrorist.BP_CounterTerrorist_C"))))

(fn `Get_GM_CounterStrike`
  (returns (NewParam :type "/Game/BluePrints/GameMode/GM_CounterStrike Object Reference"))
  (return self))

(fn `UserConstructionScript`)