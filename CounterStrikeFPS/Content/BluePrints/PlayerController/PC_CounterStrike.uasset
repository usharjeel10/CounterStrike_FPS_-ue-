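; Player controller for a Counter-Strike style game that handles team selection and pawn spawning.
; BeginPlay caches the game mode and shows the team selection widget through a client event, creating it on first use.
; Team picks pass through a server event to the game mode's RequestTeam.
; The spawnPlayer event spawns the given class at a transform, possesses it, then has the client hide the selection widget.
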(event `self.ReceiveBeginPlay`
  (`self.showHideWidget` "NewEnumerator0" true)
  (bind _newparam (message `/Game/BluePrints/Characters/Interfaces/INT_GM_CounterStrike.Get_GM_CounterStrike` (`GameplayStatics.GetGameMode`)))
  (set `self.gameMode` _newparam))

(event `showHideWidget`
  (params (widget :type "/Game/BluePrints/Characters/Enums/E_Widget Enum" :default "NewEnumerator0") (show :type Boolean))
  (`self.CL_showHideWidget` widget show))

(event `CL_showHideWidget`
  (params (NewParam :type "/Game/BluePrints/Characters/Enums/E_Widget Enum" :default "NewEnumerator0") (show :type Boolean))
  (if show
    (`self.ShowWidget` NewParam)
    (else
      (`self.HideWidget` NewParam))))

(event `selectTeam`
  (params (Class :type "Actor Class Reference"))
  (`self.SRV_SelectTeam` Class))

(event `SRV_SelectTeam`
  (params (Class :type "Actor Class Reference"))
  (`/Game/BluePrints/GameMode/GM_CounterStrike.requestTeam` (`self.gameMode`) self Class))

(event `spawnPlayer`
  (params (Class :type "Actor Class Reference") (SpawnTransform :type "Transform Structure"))
  (bind _returnvalue (`|SpawnActorFromClass` Class SpawnTransform "AdjustIfPossibleButAlwaysSpawn" "OverrideRootScale" null null))
  (bind _output_get (set `self.playerPawn` _returnvalue))
  (bind _newparam (message `/Game/BluePrints/Characters/Interfaces/INT_PlayerBase.PlayerRef` _output_get))
  (`self.Possess` _newparam)
  (`self.CL_SpawnPlayer`))

(event `CL_SpawnPlayer`
  (`self.showHideWidget` "NewEnumerator0"))

(fn `HideWidget`
  (params (widget :type "/Game/BluePrints/Characters/Enums/E_Widget Enum" :default "NewEnumerator0"))
  (switch `/Game/BluePrints/Characters/Enums/E_Widget` widget
    (:`NewEnumerator0`
      (bind _wb_teamselection (`self.WB_TeamSelection`)
        (:`then`
          (`Widget.RemoveFromParent` _wb_teamselection))
        (:`else`)))))

(fn `PC_CounterStrike`
  (returns (PlayerController :type "/Game/BluePrints/PlayerController/PC_CounterStrike Object Reference") (NewParam :type "/Game/BluePrints/PlayerController/PC_CounterStrike Object Reference"))
  (return self null))

(fn `PC_CounterStrikeFun`
  (returns (NewParam :type "/Game/BluePrints/PlayerController/PC_CounterStrike Object Reference"))
  (return self))

(fn `ShowWidget`
  (params (widget :type "/Game/BluePrints/Characters/Enums/E_Widget Enum" :default "NewEnumerator0"))
  (switch `/Game/BluePrints/Characters/Enums/E_Widget` widget
    (:`NewEnumerator0`
      (`self.WB_TeamSelection`
        (:`then`
          _)
        (:`else`
          (bind _returnvalue (`|CreateWidget` "/Game/BluePrints/UI_Widget/UI_teamSelection.UI_teamSelection_C"))
          (bind _output_get (set `self.WB_TeamSelection` _returnvalue))))
      (`UserWidget.AddToViewport` _output_get 0))))

(fn `UserConstructionScript`)