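; First-person player character that handles Enhanced Input movement, look, jump, walk and crouch, with the mesh's head bone hidden.
; Walk and crouch push or remove entries in a PlayerStates stack, whose last entry sets max speed and crouch pose.
; Non-authority instances apply changes locally and forward them through server calls.
; The airborne check only tests IsFlying, gating jump and crouch, with crouch retrying on a short delay.
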(event `self.ReceiveBeginPlay`
  (bind _newparam (message `/Game/BluePrints/Characters/Interfaces/INT_PC_counterStrike.PC_CounterStrikeFun` (`self.GetController`)))
  (`/Engine/EditorBlueprintResources/StandardMacros.IsValid` _newparam
    (:`Is Valid`
      (`EnhancedInputSubsystemInterface.AddMappingContext` (pcsubsystem `EnhancedInputLocalPlayerSubsystem` _newparam) "/Game/BluePrints/Characters/InputManager/Input.Input" 0 (struct))
      (`SkinnedMeshComponent.HideBoneByName` (`self.Mesh`) "head" "PBO_None"))))

(event `EnhancedInput|/Game/BluePrints/Characters/InputManager/movement`
  (params (ActionValue :type "Vector2D Structure") (ElapsedSeconds :type "Float (double-precision)") (TriggeredSeconds :type "Float (double-precision)") (InputAction :type "InputAction Object Reference" :default "/Game/BluePrints/Characters/InputManager/movement.movement"))
  (:`Triggered`
    (`self.AddMovementInput` (`self.GetActorForwardVector`) ActionValue_X)
    (`self.AddMovementInput` (`self.GetActorRightVector`) ActionValue_Y)))

(event `EnhancedInput|/Game/BluePrints/Characters/InputManager/LookAxis`
  (params (ActionValue :type "Vector2D Structure") (ElapsedSeconds :type "Float (double-precision)") (TriggeredSeconds :type "Float (double-precision)") (InputAction :type "InputAction Object Reference" :default "/Game/BluePrints/Characters/InputManager/LookAxis.LookAxis"))
  (:`Triggered`
    (`self.AddControllerYawInput` ActionValue_X)
    (`self.AddControllerPitchInput` ActionValue_Y)))

(event `self.ReceiveTick`
  (params (DeltaSeconds :type "Float (single-precision)"))
  (if (not (`self.f_is_not_jumping`))
    (`KismetSystemLibrary.PrintString` "In Air")))

(event `EnhancedInput|/Game/BluePrints/Characters/InputManager/crouch`
  (params (ActionValue :type Boolean) (ElapsedSeconds :type "Float (double-precision)") (TriggeredSeconds :type "Float (double-precision)") (InputAction :type "InputAction Object Reference" :default "/Game/BluePrints/Characters/InputManager/crouch.crouch"))
  (:`Triggered`
    (if (`self.f_is_not_jumping`) :!label _label
      (if ActionValue
        (`self.f_crouch` true)
        (elif (`KismetArrayLibrary.Array_Contains` (`self.playerStates`) "NewEnumerator2")
          (`self.f_crouch` false)))
      (else
        (`KismetSystemLibrary.Delay` 0.05)
        (goto _label)))))

(event `SRV_Crouch`
  (params (b_crouch :type Boolean))
  (`self.f_crouch` b_crouch))

(event `EnhancedInput|/Game/BluePrints/Characters/InputManager/walk`
  (params (ActionValue :type Boolean) (ElapsedSeconds :type "Float (double-precision)") (TriggeredSeconds :type "Float (double-precision)") (InputAction :type "InputAction Object Reference" :default "/Game/BluePrints/Characters/InputManager/walk.walk"))
  (:`Triggered`
    (if ActionValue
      (`self.f_walk` true)
      (else
        (`self.f_walk` false)))))

(event `SRV_Walk`
  (params (walk :type Boolean))
  (`self.f_walk` walk))

(event `EnhancedInput|/Game/BluePrints/Characters/InputManager/jump`
  (params (ActionValue :type Boolean) (ElapsedSeconds :type "Float (double-precision)") (TriggeredSeconds :type "Float (double-precision)") (InputAction :type "InputAction Object Reference" :default "/Game/BluePrints/Characters/InputManager/jump.jump"))
  (:`Triggered`
    (if (`self.f_is_not_jumping`)
      (`self.Jump`))))

(fn `f_crouch`
  (params (b_crouch :type Boolean))
  (locals (Iscrouching :type Boolean))
  (bind _playerstates (`self.playerStates`))
  (bind _output_get (set `local.Iscrouching` b_crouch))
  (`/Engine/EditorBlueprintResources/ActorMacros.Switch Has Authority`
    (:`Authority`
      _)
    (:`Remote`
      (`self.SRV_Crouch` _output_get)))
  (if (`local.Iscrouching`)
    (`self.Crouch`)
    (`KismetArrayLibrary.Array_Set` _playerstates (+ (`KismetArrayLibrary.Array_LastIndex` _playerstates) 1) "NewEnumerator2" true)
    (`self.f_setMovementSpeed`)
    (else
      (`self.UnCrouch`)
      (`KismetArrayLibrary.Array_RemoveItem` (`self.playerStates`) "NewEnumerator2")
      (`self.f_setMovementSpeed`))))

(fn `f_is_not_jumping`
  (returns (ReturnValue :type Boolean))
  (return (not (`NavMovementComponent.IsFlying` (`self.CharacterMovement`)))))

(fn `f_setMovementSpeed`
  (bind _playerstates (`self.playerStates`))
  (bind _playerstates_2 (`self.playerStates`))
  (if (`|EnumEquality` (`|GetArrayItem` _playerstates_2 (`KismetArrayLibrary.Array_LastIndex` _playerstates_2)) "NewEnumerator2")
    (`self.Crouch`)
    (else
      (`self.UnCrouch`)))
  (set `CharacterMovementComponent.MaxWalkSpeed` (select `/Game/BluePrints/Characters/Enums/E_PlayerState` (`|GetArrayItem` _playerstates (`KismetArrayLibrary.Array_LastIndex` _playerstates)) :`NewEnumerator0` (`self.runSpeed`) :`NewEnumerator1` (`self.walkSpeed`) :`NewEnumerator2` (`self.CrouchSpeed`) :!type "Float (single-precision)") (`self.CharacterMovement`)))

(fn `f_walk`
  (params (walk :type Boolean))
  (locals (Iscrouching :type Boolean) (Iswalking :type Boolean))
  (bind _playerstates (`self.playerStates`))
  (bind _output_get (set `local.Iswalking` walk))
  (`/Engine/EditorBlueprintResources/ActorMacros.Switch Has Authority`
    (:`Authority`
      _)
    (:`Remote`
      (`self.SRV_Walk` _output_get)))
  (if (`local.Iswalking`)
    (`KismetArrayLibrary.Array_Set` _playerstates (+ (`KismetArrayLibrary.Array_LastIndex` _playerstates) 1) "NewEnumerator1" true)
    (`self.f_setMovementSpeed`)
    (else
      (`KismetArrayLibrary.Array_RemoveItem` (`self.playerStates`) "NewEnumerator1")
      (`self.f_setMovementSpeed`))))

(fn `PlayerRef`
  (returns (NewParam :type "/Game/BluePrints/Characters/BP_PlayerClass Object Reference"))
  (return self))

(fn `UserConstructionScript`)